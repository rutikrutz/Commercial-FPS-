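; Zombie enemy Blueprint that chases the player, takes bone-specific damage and ragdolls on death.
; Every Tick it reissues AI MoveTo toward the player character and calls Die once EnemyHealth reaches zero or below.
; The ItakeDamage event subtracts incoming damage, adds a fixed head-bone penalty and only prints debug labels for other matched bones.
; Die enables mesh physics and disables capsule collision.
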(event EventTick
  (params (DeltaSeconds :type Float%20%28single-precision%29))
  ;[1 1 1] Tick
  (Utilities|FlowControl|Sequence
    (:then_0
      (AI|AIMoveTo self "0, 0, 0" (Game|GetPlayerCharacter 0) 5.0 false))
    (:then_1
      (if (<= (Variables|Default|Getenemy_health) 0)
        (CallFunction|Die)))))

(event EventItakeDamage
  (params (Bone%20name :type Name) (Damage :type Integer))
  (Utilities|FlowControl|Sequence
    (:then_0
      ;[1 1 1] Damage
      (Variables|Default|Setenemy_health (- (Variables|Default|Getenemy_health) (Math|Float|Truncate (Math|Conversions|ToFloat(Integer) Damage)))))
    (:then_1
      (if (Utilities|Name|Equal(Name) Bone%20name "cc_base_head")
        (Development|PrintString "head")
        (Variables|Default|Setenemy_health (- (Variables|Default|Getenemy_health) 200))
        (Development|PrintString "headShot")))
    (:then_2
      (if (Utilities|Name|Equal(Name) Bone%20name "cc_base_hip")
        (Development|PrintString "pelvis")))
    (:then_3
      (if (Utilities|Name|Equal(Name) Bone%20name "cc_base_r_forearm")
        (Development|PrintString "Right Arm")))
    (:then_4
      (if (Utilities|Name|Equal(Name) Bone%20name "cc_base_l_clavicle")
        (Development|PrintString "leftarm")))))

(event EventDie
  ;[1 1 1] Ragdoll Mode ON
  (Physics|SetSimulatePhysics (Variables|Character|GetMesh) true)
  (Collision|SetCollisionEnabled (Variables|Default|GetCapsuleComponent) "NoCollision"))

(fn ConstructionScript
  (|CallParentFunction))