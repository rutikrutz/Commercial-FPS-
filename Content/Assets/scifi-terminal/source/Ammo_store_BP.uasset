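; Ammo store actor that shows a floating label and tracks whether the player stands in its reloading area.
; The Sphere shows the label when the player enters and hides it when any overlap ends, because the exit check compares the overlapped component to the player.
; Tick rotates the label toward the player's mesh.
; ReloadingArea sets InZone on player entry and exit with debug prints; no reload logic lives here.
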(event OnComponentBeginOverlap(Sphere)
  (params (OverlappedComponent :type Primitive%20Component%20Object%20Reference) (OtherActor :type Actor%20Object%20Reference) (OtherComp :type Primitive%20Component%20Object%20Reference) (OtherBodyIndex :type Integer) (bFromSweep :type Boolean) (SweepResult :type Hit%20Result%20Structure%20%28by%20ref%29))
  (if (== OtherActor (Game|GetPlayerCharacter 0))
    (Rendering|SetVisibility (Variables|Default|GetAmmo%20Store%20label) true false)))

(event OnComponentEndOverlap(Sphere)
  (params (OverlappedComponent :type Primitive%20Component%20Object%20Reference) (OtherActor :type Actor%20Object%20Reference) (OtherComp :type Primitive%20Component%20Object%20Reference) (OtherBodyIndex :type Integer))
  (if (not (== OverlappedComponent (Game|GetPlayerCharacter 0)))
    (Rendering|SetVisibility (Variables|Default|GetAmmo%20Store%20label) false false)))

(event OnComponentBeginOverlap(reloadingarea)
  (params (OverlappedComponent :type Primitive%20Component%20Object%20Reference) (OtherActor :type Actor%20Object%20Reference) (OtherComp :type Primitive%20Component%20Object%20Reference) (OtherBodyIndex :type Integer) (bFromSweep :type Boolean) (SweepResult :type Hit%20Result%20Structure%20%28by%20ref%29))
  (if (== OtherActor (Game|GetPlayerCharacter 0))
    (Variables|Default|Setin%20Zone? true)
    (Development|PrintString "enter")))

(event OnComponentEndOverlap(reloadingarea)
  (params (OverlappedComponent :type Primitive%20Component%20Object%20Reference) (OtherActor :type Actor%20Object%20Reference) (OtherComp :type Primitive%20Component%20Object%20Reference) (OtherBodyIndex :type Integer))
  (if (== OtherActor (Game|GetPlayerCharacter 0))
    (Variables|Default|Setin%20Zone? false)
    (Development|PrintString "exit")))

(event EventBeginPlay)

(event Collision|EventActorBeginOverlap
  (params (OtherActor :type Actor%20Object%20Reference)))

(event EventTick
  (params (DeltaSeconds :type Float%20%28single-precision%29))
  (Transformation|SetRelativeRotation (Variables|Default|GetAmmo%20Store%20label) (Math|Rotator|FindLookatRotation (Transformation|GetWorldLocation (Variables|Default|GetAmmo%20Store%20label)) (Transformation|GetWorldLocation (Variables|/Script/Engine.Character|GetMesh (Game|GetPlayerCharacter 0)))) false false))

(fn ConstructionScript)